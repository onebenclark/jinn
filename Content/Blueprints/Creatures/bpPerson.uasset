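; bpPerson is a person creature with a modular body and a dialog component.
; The construction script offsets the target and mesh components, slaves feet, legs, torso and hands to the main mesh via master pose, and snaps the head attachment to headSocket.
; It also constructs a placeholder greeting dialog node with one response as the initial dialog.
; The event graph holds only disabled stub events.
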(event EventBeginPlay)

(event Collision|EventActorBeginOverlap
  (params (OtherActor :type Actor%20Object%20Reference)))

(event EventTick
  (params (DeltaSeconds :type Float%20%28single-precision%29)))

(fn ConstructionScript
  (bind _dialogcomponent (Variables|Default|GetDialogComponent))
  (Transformation|SetRelativeLocation (Variables|Default|GetTargetComponent) "0, 0,40.000000" false false)
  (Transformation|SetRelativeLocation (Variables|Default|GetMeshComponent) "0, 0,-90.000000" false false)
  (Class|SkinnedMeshComponent|SetMasterPoseComponent (Variables|Default|GetFeet) (Variables|Default|GetMeshComponent) false)
  (Transformation|AttachComponentToComponent (Variables|Default|GetHeadAttachment) (Variables|Default|GetMeshComponent) "headSocket" "SnapToTarget" "SnapToTarget" "SnapToTarget" true)
  (bind _returnvalue (Game|ConstructObjectfromClass "/Script/Jinn.DialogNode" _dialogcomponent))
  (bind _output_get (Variables|/Script/Jinn.DialogComponent|SetInitialDialogNode _dialogcomponent _returnvalue))
  (Variables|/Script/Jinn.DialogNode|SetDialogText _output_get "Hi me")
  (bind _returnvalue_2 (Game|ConstructObjectfromClass "/Script/Jinn.DialogResponse" _output_get))
  (Variables|/Script/Jinn.DialogResponse|SetResponseText _returnvalue_2 "Hello You")
  (Utilities|Array|Add (Variables|/Script/Jinn.DialogNode|GetResponses _output_get) _returnvalue_2))