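; Enemy creature Blueprint with modular body meshes, a heavy axe and a head attachment.
; When pawn sensing sees a creature of an opposing, non-neutral allegiance and no valid target is held, it takes that creature as Target and switches State to Agro.
; The construction script offsets the mesh and target component, slaves body parts to the main mesh as master pose, and attaches the axe and head piece to sockets.
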(event OnSeePawn(PawnSensing)
  (params (Pawn :type Pawn%20Object%20Reference))
  (if (not (Utilities|IsValid (Variables|Default|GetTarget)))
    (bind _ascreature (Utilities|Casting|CastToCreature Pawn))
    (if (and (Utilities|Enum|NotEqual(Enum) (Variables|/Script/Jinn.Creature|GetAllegiance _ascreature) "Neutral") (Utilities|Enum|NotEqual(Enum) (Variables|/Script/Jinn.Creature|GetAllegiance _ascreature) (Variables|Default|GetAllegiance)))
      (Variables|Default|SetTarget _ascreature)
      (Variables|Default|SetState "Agro"))))

(event EventBeginPlay)

(event EventTick
  (params (DeltaSeconds :type Float%20%28single-precision%29)))

(fn ConstructionScript
  (Transformation|SetRelativeLocation (Variables|Default|GetTargetComponent) "0, 0,40.000000" false false)
  (Transformation|SetRelativeLocation (Variables|Default|GetMeshComponent) "0, 0,-90.000000" false false)
  (Class|SkinnedMeshComponent|SetMasterPoseComponent (Variables|Default|GetTorso) (Variables|Default|GetMeshComponent) false)
  (Transformation|AttachComponentToComponent (Variables|Default|GetSK_Blade_HeavyAxe) (Variables|Default|GetMeshComponent) "hand_rSocket" "KeepRelative" "KeepRelative" "KeepRelative" true)
  (Transformation|AttachComponentToComponent (Variables|Default|GetHeadAttachment) (Variables|Default|GetMeshComponent) "headSocket" "SnapToTarget" "SnapToTarget" "SnapToTarget" true)
  (Transformation|SetRelativeLocation (Variables|Default|GetTargetComponent) "0, 0,40.000000" false false)
  (Transformation|SetRelativeLocation (Variables|Default|GetMeshComponent) "0, 0,-90.000000" false false))