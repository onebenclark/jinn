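; Action Blueprint that launches a homing missile from the caller at a target.
; ActionEffects runs the parent effects, then spawns a projectile SpawnDistance ahead of the caller with zero rotation.
; If it is a bpMissle, it receives the Target and Source, and its projectile movement homes on the target's capsule.
; An invalid target only prints a debug message, and the action still returns true.
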(fn ActionEffects
  (params (Caller :type Creature%20Object%20Reference) (Target :type Creature%20Object%20Reference))
  (|CallParentFunction 0 0)
  (Utilities|IsValid Target
    (:Is%20Valid
      (bind _returnvalue (Class|Action|Spawn (+ (Transformation|GetActorLocation Caller) (* (Transformation|GetActorForwardVector Caller) (Variables|Default|GetSpawnDistance))) "0, 0, 0"))
      (bind _asbp_missle (Utilities|Casting|CastTobpMissle _returnvalue)
        (:then
          (Variables|/Script/Jinn.Missle|SetTarget _asbp_missle Target)
          (Variables|/Script/Jinn.Missle|SetSource _asbp_missle Caller)
          (Variables|/Script/Engine.ProjectileMovementComponent|SetHomingTargetComponent (Variables|/Script/Jinn.Missle|GetProjectileMovementComponent _asbp_missle) (Variables|/Script/Jinn.Creature|GetCapsule Target)))
        (:CastFailed
          _)))
    (:Is%20Not%20Valid
      (Development|PrintString 0 "No Target Input" false)))
  (return true))