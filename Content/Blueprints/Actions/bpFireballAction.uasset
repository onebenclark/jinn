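; Fireball action that launches a homing missile from the caller toward a chosen target.
; ActionEffects spawns the projectile ahead of the caller, casts it to bpMissle and assigns its source and target.
; Homing locks onto the Capsule of the target, which must be an ActionPlacementActor.
; The action completes immediately after setup or on an invalid target, but a failed cast exits without setting Complete.
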(fn ActionEffects
  (params (Caller :type Creature%20Object%20Reference) (Target :type Actor%20Object%20Reference))
  (if (Utilities|IsValid Target)
    (bind _returnvalue (Class|Action|Spawn (+ (Transformation|GetActorLocation Caller) (* (Transformation|GetActorForwardVector Caller) (Variables|Default|GetSpawnDistance))) "0, 0, 0"))
    (bind _asbp_missle (Utilities|Casting|CastTobpMissle _returnvalue))
    (Variables|/Script/Jinn.Missle|SetTarget _asbp_missle Target)
    (Variables|/Script/Jinn.Missle|SetSource _asbp_missle Caller)
    (bind _asaction_placement_actor (Utilities|Casting|CastToActionPlacementActor Target))
    (Variables|/Script/Engine.ProjectileMovementComponent|SetHomingTargetComponent (Variables|/Script/Jinn.Missle|GetProjectileMovementComponent _asbp_missle) (Variables|/Script/Jinn.ActionPlacementActor|GetCapsule _asaction_placement_actor))
    (Variables|Default|SetComplete true)
    (return true)
    (else
      (Variables|Default|SetComplete true)
      (return true))))