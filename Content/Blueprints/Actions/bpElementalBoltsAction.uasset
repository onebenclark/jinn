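; Combat action that conjures a volley of elemental bolts around the caller and launches them as homing missiles at a target.
; Each ActionEffects call advances a stage, spawning the next fire, lightning or ice bolt along an arc in the caller's right/up plane.
; Spawned bolts record the caller as source and wait in an array.
; The final stage assigns each bolt's target and homing component, clears the array and completes the action.
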(fn ActionEffects
  (params (Caller :type Creature%20Object%20Reference) (Target :type Creature%20Object%20Reference))
  (bind _returnvalue (Transformation|GetActorRightVector Caller))
  (bind _returnvalue_2 (Transformation|GetActorUpVector Caller))
  (bind _returnvalue_3 (Transformation|GetActorLocation Caller))
  (bind _spawndistance (Variables|Default|GetSpawnDistance))
  (bind _returnvalue_4 (Math|Vector|NegateVector _returnvalue))
  (Utilities|IsValid Target
    (:Is%20Valid
      (switch int (Variables|Default|GetStage)
        (:0
          (LocalVariables|SetSpawnLocation (+ _returnvalue_3 (* _returnvalue _spawndistance)))
          (Variables|Default|SetSpawnedClass "/Game/Blueprints/bpFireBolt.bpFireBolt_C")
          (Math|Integer|IncrementInt (Variables|Default|GetStage)
            (:%20%20
              _)))
        (:1
          (LocalVariables|SetSpawnLocation (+ _returnvalue_3 (* (Math|Vector|Normalize (+ _returnvalue _returnvalue_2)) _spawndistance)))
          (Variables|Default|SetSpawnedClass "/Game/Blueprints/bpLightningOrb.bpLightningOrb_C")
          (Math|Integer|IncrementInt (Variables|Default|GetStage)
            (:%20%20
              _)))
        (:2
          (LocalVariables|SetSpawnLocation (+ _returnvalue_3 (* _returnvalue_2 _spawndistance)))
          (Variables|Default|SetSpawnedClass "/Game/Blueprints/bpIceBolt.bpIceBolt_C")
          (Math|Integer|IncrementInt (Variables|Default|GetStage)
            (:%20%20
              _)))
        (:3
          (LocalVariables|SetSpawnLocation (+ _returnvalue_3 (* (Math|Vector|Normalize (+ _returnvalue_4 _returnvalue_2)) _spawndistance)))
          (Variables|Default|SetSpawnedClass "/Game/Blueprints/bpFireBolt.bpFireBolt_C")
          (Math|Integer|IncrementInt (Variables|Default|GetStage)
            (:%20%20
              _)))
        (:4
          (LocalVariables|SetSpawnLocation (+ _returnvalue_3 (* _returnvalue_4 _spawndistance)))
          (Variables|Default|SetSpawnedClass "/Game/Blueprints/bpLightningOrb.bpLightningOrb_C")
          (Math|Integer|IncrementInt (Variables|Default|GetStage)
            (:%20%20
              _)))
        (:5
          (LocalVariables|SetSpawnLocation (+ _returnvalue_3 (* (Math|Vector|Normalize (+ (Math|Vector|NegateVector _returnvalue_2) _returnvalue_4)) _spawndistance)))
          (Variables|Default|SetSpawnedClass "/Game/Blueprints/bpIceBolt.bpIceBolt_C")
          (Math|Integer|IncrementInt (Variables|Default|GetStage)
            (:%20%20
              _)))
        (:6
          (Variables|Default|SetStage 0)
          (Variables|Default|SetComplete true)
          (for _array_element (Variables|Default|GetBolts)
            (Variables|/Script/Jinn.Missle|SetTarget _array_element Target)
            (Variables|/Script/Engine.ProjectileMovementComponent|SetHomingTargetComponent (Variables|/Script/Jinn.Missle|GetProjectileMovementComponent _array_element) (Variables|/Script/Jinn.Creature|GetCapsule Target)))
          (Utilities|Array|Clear (Variables|Default|GetBolts))
          (return true)))
      (bind _returnvalue_5 (Class|Action|Spawn (LocalVariables|GetSpawnLocation) "0, 0, 0"))
      (bind _asbp_missle (Utilities|Casting|CastTobpMissle _returnvalue_5))
      (Utilities|Array|Add (Variables|Default|GetBolts) _asbp_missle)
      (Variables|/Script/Jinn.Missle|SetSource _asbp_missle Caller)
      (return true))
    (:Is%20Not%20Valid
      (return true))))