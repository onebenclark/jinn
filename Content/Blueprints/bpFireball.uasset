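; Fireball projectile actor that destroys its designated Target actor on overlap, ignoring all other actors.
; On that hit it swaps its particle system to an enlarged explosion, stops projectile movement, destroys the target and hides its sphere.
; A pending-destroy flag then lets Tick accumulate time and destroy the fireball about three seconds later, leaving time for the explosion effect.
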(event EventBeginPlay
  (|CallParentFunction) ; This node is disabled and will not be called.\nDrag off pins to build functionality.
)

(event Collision|EventActorBeginOverlap
  (params (OtherActor :type Actor%20Object%20Reference))
  (bind _target (Variables|Default|GetTarget))
  (bind _particlesystem (Variables|Default|GetParticleSystem))
  (if (not (== OtherActor self))
    (if (== OtherActor _target)
      (Effects|Components|ParticleSystem|SetTemplate _particlesystem "/Game/StarterContent/Particles/P_Explosion.P_Explosion")
      (Transformation|SetWorldScale3D _particlesystem "2.000000,2.000000,2.000000")
      (Components|Movement|StopMovementImmediately (Variables|Default|GetProjectileMovementComponent))
      (Actor|DestroyActor _target)
      (Rendering|SetVisibility (Variables|Default|GetSphere) false false)
      (Variables|Default|SetToBeDestroyed true))))

(event EventTick
  (params (DeltaSeconds :type Float%20%28single-precision%29))
  (if (Variables|Default|GetToBeDestroyed)
    (bind _output_get (Variables|Default|SetTimeSinceDestroyPending (+ (Variables|Default|GetTimeSinceDestroyPending) DeltaSeconds)))
    (if (> _output_get 3.0)
      (Actor|DestroyActor))))

(fn ConstructionScript
  (|CallParentFunction))