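; Action Blueprint that launches a projectile from the caller toward a target.
; ActionEffects runs the parent effects, then, if the target is valid, spawns an actor at a raised point in front of the caller.
; If that actor is a bpProjectile, its movement velocity is set once along the normalized direction to the target's location at a fixed speed.
; The function returns true even when no valid target exists.
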(fn ActionEffects
  (params (Caller :type Creature%20Object%20Reference) (Target :type Creature%20Object%20Reference))
  (bind _returnvalue (Transformation|GetActorLocation Caller))
  (bind _returnvalue_2 (Transformation|GetActorForwardVector Caller))
  (bind _spawndistance (Variables|Default|GetSpawnDistance))
  (bind _returnvalue_3 (* _returnvalue_2 _spawndistance))
  (bind _returnvalue_4 (+ _returnvalue _returnvalue_3 "0,0,60.000000"))
  (|CallParentFunction 0 0)
  (Utilities|IsValid Target
    (:Is%20Valid
      (bind _returnvalue_5 (Class|Action|Spawn _returnvalue_4 "0, 0, 0"))
      (bind _asbp_projectile (Utilities|Casting|CastTobpProjectile _returnvalue_5)
        (:then
          (Variables|/Script/Engine.MovementComponent|SetVelocity (Variables|/Script/Jinn.Projectile|GetProjectileMovementComponent _asbp_projectile) (* (Math|Vector|Normalize (- (Transformation|GetActorLocation Target) _returnvalue_4)) 3e+03)))
        (:CastFailed
          _)))
    (:Is%20Not%20Valid
      _))
  (return true))