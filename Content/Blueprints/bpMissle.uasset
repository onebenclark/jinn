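; Missile actor that damages one assigned Target when it overlaps it.
; Overlaps with any other actor are ignored; a hit on Target applies Damage, credited to the Source actor and its controller, then destroys the missile.
; The graph holds no movement or homing logic and does not set Target or Source; BeginPlay, Tick and the construction script are empty.
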(event EventBeginPlay)

(event Collision|EventActorBeginOverlap
  (params (OtherActor :type Actor%20Object%20Reference))
  (bind _source (Variables|Default|GetSource))
  (if (not (== OtherActor self))
    (if (== OtherActor (Variables|Default|GetTarget))
      (Game|Damage|ApplyDamage (Variables|Default|GetTarget) (Variables|Default|GetDamage) (Pawn|GetController _source) _source "/Script/Engine.DamageType")
      (Actor|DestroyActor))))

(event EventTick
  (params (DeltaSeconds :type Float%20%28single-precision%29)))

(fn ConstructionScript)