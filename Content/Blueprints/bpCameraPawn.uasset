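; Camera pawn with a spring-arm camera and an action-aiming widget that follows the view direction.
; Each Tick places the widget a fixed distance from the root along the camera's flattened forward vector, slightly below root height.
; The widget is pitched to lie horizontal, with its roll derived from the camera's yaw so it turns with the view.
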(event EventBeginPlay)

(event Collision|EventActorBeginOverlap
  (params (OtherActor :type Actor%20Object%20Reference)))

(event EventTick
  (params (DeltaSeconds :type Float%20%28single-precision%29))
  (bind _rootcomponent (Variables|Transformation|GetRootComponent))
  (bind _camera (Variables|Default|GetCamera))
  (bind _returnvalue (Transformation|GetWorldLocation _rootcomponent))
  (bind _returnvalue_2 (Math|Vector|GetForwardVector _camera))
  (bind _returnvalue_3 (Class|KismetMathLibrary|VectorNormal2D _returnvalue_2 0.0001))
  (bind _returnvalue_4 (* _returnvalue_3 2.5e+02))
  (bind _returnvalue_5 (+ _returnvalue _returnvalue_4))
  (bind (_x _y _z) (Math|Vector|BreakVector _returnvalue_5))
  (Transformation|SetWorldLocationAndRotation (Variables|Default|GetActionAimingWidget) (Math|Vector|MakeVector _x _y (- _z 7e+01)) (Math|Rotator|MakeRotator (+ (* (.Yaw (Math|Rotator|BreakRotator (Math|Rotator|MakeRotationfromAxes _returnvalue_2 "0, 0, 0" "0, 0, 0"))) -1.0) 1.8e+02) 9e+01 0.0) false false))

(fn ConstructionScript)