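; An AI condition check that reports whether a Creature's attack action is available.
; It casts the controlled pawn to Creature and looks up the action component's AttackAction in its ActionMap.
; A valid entry passes only when its cooldown is exactly zero, while a missing or invalid entry counts as available.
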(fn PerformConditionCheckAI
  (params (OwnerController :type AI%20Controller%20Object%20Reference) (ControlledPawn :type Pawn%20Object%20Reference))
  (bind _ascreature (Utilities|Casting|CastToCreature ControlledPawn))
  (if (.ReturnValue (Utilities|Map|Find (Variables|/Script/Jinn.ActionComponent|GetActionMap (Variables|/Script/Jinn.Creature|GetActionComponent _ascreature)) (Variables|/Script/Jinn.ActionComponent|GetAttackAction (Variables|/Script/Jinn.Creature|GetActionComponent _ascreature))))
    (Utilities|IsValid (.Value (Utilities|Map|Find (Variables|/Script/Jinn.ActionComponent|GetActionMap (Variables|/Script/Jinn.Creature|GetActionComponent _ascreature)) (Variables|/Script/Jinn.ActionComponent|GetAttackAction (Variables|/Script/Jinn.Creature|GetActionComponent _ascreature))))
      (:Is%20Valid
        (return (== (Variables|/Script/Jinn.Action|GetCooldown (.Value (Utilities|Map|Find (Variables|/Script/Jinn.ActionComponent|GetActionMap (Variables|/Script/Jinn.Creature|GetActionComponent _ascreature)) (Variables|/Script/Jinn.ActionComponent|GetAttackAction (Variables|/Script/Jinn.Creature|GetActionComponent _ascreature))))) 0.0)))
      (:Is%20Not%20Valid
        _)))
  (return true))