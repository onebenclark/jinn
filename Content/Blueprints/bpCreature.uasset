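; Creature Blueprint that assembles a modular skeletal character with equipment and status effects.
; The construction script positions the target and mesh components, slaves torso, legs, feet and hands to the main mesh via master pose, and snaps the head attachment to its socket.
; BeginPlay takes the weapon mesh from an instance of the RightHandEquipment class, attaches the weapon to the right-hand socket, and unconditionally adds a poison status effect.
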(event EventBeginPlay
  (bind _righthandequipment (Variables|Default|GetRightHandEquipment))
  (bind _righthandweapon (Variables|Default|GetRightHandWeapon))
  (if (Utilities|IsValidClass _righthandequipment)
    (bind _returnvalue (Game|ConstructObjectfromClass _righthandequipment self))
    (Class|SkinnedMeshComponent|SetSkeletalMesh _righthandweapon (Variables|/Script/Jinn.Item|GetMesh _returnvalue) true))
  (Transformation|AttachComponentToComponent _righthandweapon (Variables|Default|GetMeshComponent) "hand_rSocket" "KeepRelative" "KeepRelative" "KeepRelative" true)
  (bind _returnvalue_2 (Game|ConstructObjectfromClass "/Game/Blueprints/bpPoisonEffect.bpPoisonEffect_C" self))
  (Utilities|Array|Add (Variables|Default|GetStatusEffects) _returnvalue_2))

(event Collision|EventActorBeginOverlap
  (params (OtherActor :type Actor%20Object%20Reference)))

(event EventTick
  (params (DeltaSeconds :type Float%20%28single-precision%29)))

(fn ConstructionScript
  (Transformation|SetRelativeLocation (Variables|Default|GetTargetComponent) "0, 0,40.000000" false false)
  (Transformation|SetRelativeLocation (Variables|Default|GetMeshComponent) "0, 0,-90.000000" false false)
  (Class|SkinnedMeshComponent|SetMasterPoseComponent (Variables|Default|GetTorso) (Variables|Default|GetMeshComponent) false)
  (Transformation|AttachComponentToComponent (Variables|Default|GetHeadAttachment) (Variables|Default|GetMeshComponent) "headSocket" "SnapToTarget" "SnapToTarget" "SnapToTarget" true))