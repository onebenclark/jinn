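; Status effect Blueprint that lowers an affected creature's accuracy while it is active.
; On start it subtracts half of the creature's base Accuracy from EffectiveAccuracy in its StatsComponent, and on end it adds half back.
; Both steps read base Accuracy at the moment they run rather than storing the applied amount.
; The recurring effects event is empty.
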(event EventBPStart
  (params (AffectedCreature :type Creature%20Object%20Reference))
  (bind _statscomponent (Variables|/Script/Jinn.Creature|GetStatsComponent AffectedCreature))
  (Variables|/Script/Jinn.StatsComponent|SetEffectiveAccuracy _statscomponent (- (Variables|/Script/Jinn.StatsComponent|GetEffectiveAccuracy _statscomponent) (* (Variables|/Script/Jinn.StatsComponent|GetAccuracy _statscomponent) 0.5))))

(event EventBPEnd
  (params (AffectedCreature :type Creature%20Object%20Reference))
  (bind _statscomponent (Variables|/Script/Jinn.Creature|GetStatsComponent AffectedCreature))
  (Variables|/Script/Jinn.StatsComponent|SetEffectiveAccuracy _statscomponent (+ (Variables|/Script/Jinn.StatsComponent|GetEffectiveAccuracy _statscomponent) (* (Variables|/Script/Jinn.StatsComponent|GetAccuracy _statscomponent) 0.5))))

(event EventBPRecurringEffects
  (params (AffectedCreature :type Creature%20Object%20Reference)))